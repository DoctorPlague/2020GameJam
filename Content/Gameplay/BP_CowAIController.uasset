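; AI controller for a cow that makes its pawn wander to random reachable points nearby.
; While idle, Tick accumulates a cooldown timer, then sets IsWandering and calls AIMoveTo.
; Only a successful move clears IsWandering, so a failed move or point search halts wandering.
; The timer is never reset, so later moves skip the cooldown; the Wander function is an empty stub.
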(event EventBeginPlay)

(event EventTick
  (params (DeltaSeconds :type Float%20%28single-precision%29))
  (bind _returnvalue (Pawn|GetControlledPawn))
  (bind _returnvalue_2 (Transformation|GetActorLocation _returnvalue))
  (bind (_randomlocation _returnvalue_3) (AI|Navigation|GetRandomReachablePointinRadius _returnvalue_2 1e+03 0 "/Script/NavigationSystem.RecastFilter_UseDefaultArea"))
  (if (not (Variables|Default|GetIsWandering))
    ;[1 1 1] Incrmeent timer
    (Variables|Default|SetWanderCooldownTimer (+ (Variables|Default|GetWanderCooldownTimer) (Utilities|Time|GetWorldDeltaSeconds)))
    (if (>= (Variables|Default|GetWanderCooldownTimer) (Variables|Default|GetWanderCooldown))
      (Variables|Default|SetIsWandering true)
      (if _returnvalue_3
        (AI|AIMoveTo (Pawn|GetControlledPawn) _randomlocation 0 2.5e+02 false
          (:OnSuccess
            (Variables|Default|SetIsWandering false)))))))

(fn ConstructionScript)

(fn Wander)