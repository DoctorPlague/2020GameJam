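; Gate actor Blueprint that fades an interact prompt label according to the player's distance from it.
; On BeginPlay it caches the label from the InteractPrompt widget component and starts a fast looping timer.
; Each timer tick maps player distance to label opacity with a clamped range, so the prompt is opaque up close and fades out farther away.
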(event Custom|EventInteractLabelVisibility
  (Widget|SetRenderOpacity (Variables|Default|GetInteractLabel) (Math|Float|MapRangeClamped (Transformation|GetDistanceTo (Game|GetPlayerCharacter 0)) 5e+01 1.5e+02 1.0 0.0)))

(event EventBeginPlay
  (bind _asinteract_prompt (Utilities|Casting|CastToInteractPrompt (UserInterface|GetUserWidgetObject (Variables|Default|GetInteractPrompt))))
  (Variables|Default|SetInteractLabel (Variables|/Game/UI/InteractPrompt.InteractPrompt_C|GetLabel _asinteract_prompt))
  (Utilities|Time|SetTimerbyEvent (delegate Custom|EventInteractLabelVisibility) 0.05 true))

(fn ConstructionScript)