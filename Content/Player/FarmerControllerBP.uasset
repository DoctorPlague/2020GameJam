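; Player controller for the farmer in a cow-milking game, owning the HUD, end screen, and dialogue and response wheel widgets.
; BIon events update milk progress and switch widgets between game views, while mouse clicks feed the dialogue wheel.
; Interacting with a cow starts a simple move to its front, then Tick lerps the farmer's rotation to face it on arrival.
; The L key directly triggers a "Cow die" game loss.
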(event EventBeginPlay
  (bind _returnvalue (UserInterface|CreateWidget "/Game/UI/PlayerHUD.PlayerHUD_C" self))
  (bind _output_get (Variables|Default|SetPlayerHud _returnvalue))
  (UserInterface|Viewport|AddtoViewport _output_get 0)
  (Default|SetPailCount _returnvalue (Variables|Default|GetiNumberOfCowsNeeded)))

(event EventTick
  (params (DeltaSeconds :type Float%20%28single-precision%29))
  (CallFunction|ProcessMovetoFrontOfCow))

(event EventBIonInteractwithCow
  (params (_Cow :type Cow%20Object%20Reference))
  (bind _ascow_bp (Utilities|Casting|CastToCowBP _Cow))
  (bind _output_get (Variables|Default|SetClosestCow _ascow_bp))
  (Widget|SetRenderOpacity (Variables|/Game/Gameplay/CowBP.CowBP_C|GetInteractLabel _output_get) 0.0)
  (AI|Navigation|SimpleMovetoLocation self (+ (Transformation|GetActorLocation _ascow_bp) (* (Transformation|GetActorForwardVector _ascow_bp) (Variables|Default|GetTargetDistanceInFrontOfCow))))
  (Variables|Default|SetTargetDestination (+ (Transformation|GetActorLocation _ascow_bp) (* (Transformation|GetActorForwardVector _ascow_bp) (Variables|Default|GetTargetDistanceInFrontOfCow))))
  (Variables|Default|SetHasReachedDestination false))

(event EventBIonGameLost)

(event EventBIonAddSuccessfulCow
  (params (_PercentageComplete :type Float%20%28single-precision%29))
  (bind _playerhud (Variables|Default|GetPlayerHud))
  (Default|CompletedNewPail _playerhud)
  (Default|SetMilkPercentage _playerhud _PercentageComplete))

(event EventBIonShowEndScreen
  (params (_Status :type String) (_Reason :type String))
  (bind _returnvalue (UserInterface|CreateWidget "/Game/UI/FailScreen.FailScreen_C" self))
  (Default|SetInfo _returnvalue _Status _Reason)
  (UserInterface|Viewport|AddtoViewport _returnvalue 0))

(event EventBIonStartConversationView
  (bind _dialoguewheelwidget (Variables|Default|GetDialogueWheelWidget)
    (:then
      (Widget|RemovefromParent _dialoguewheelwidget))
    (:else
      _))
  (Variables|Default|SetDialoguePlaying false)
  (bind _reponsewheelwidget (Variables|Default|GetReponseWheelWidget)
    (:then
      (Widget|RemovefromParent _reponsewheelwidget))
    (:else)))

(event EventBIonSpeechGameView
  (bind _dialoguewheelwidget (Variables|Default|GetDialogueWheelWidget)
    (:then
      _)
    (:else
      (bind _returnvalue (UserInterface|CreateWidget "/Game/UI/DialogueWheel.DialogueWheel_C" self))
      (bind _output_get (Variables|Default|SetDialogueWheelWidget _returnvalue))))
  (UserInterface|Viewport|AddtoViewport _output_get 0)
  (Variables|Default|SetDialoguePlaying true))

(event EventBIonPlayerView
  (params (_ExpectedReaction :type EReactionType%20Enum :default "E_ANGRY"))
  (Variables|Default|GetReponseWheelWidget
    (:then
      _)
    (:else
      (bind _returnvalue (UserInterface|CreateWidget "/Game/UI/ResponseWheel.ResponseWheel_C" self))
      (bind _output_get (Variables|Default|SetReponseWheelWidget _returnvalue))
      (Default|SetWinReaction _output_get _ExpectedReaction)))
  (UserInterface|Viewport|AddtoViewport (Variables|Default|GetReponseWheelWidget) 0))

(event EventBIonStartInteractComplete
  (bind _dialoguewheelwidget (Variables|Default|GetDialogueWheelWidget)
    (:then
      (Widget|RemovefromParent _dialoguewheelwidget))
    (:else
      _))
  (Variables|Default|SetDialoguePlaying false)
  (bind _reponsewheelwidget (Variables|Default|GetReponseWheelWidget)
    (:then
      (Widget|RemovefromParent _reponsewheelwidget))
    (:else)))

(event EventBIonStartCowView
  (bind _dialoguewheelwidget (Variables|Default|GetDialogueWheelWidget)
    (:then
      (Widget|RemovefromParent _dialoguewheelwidget))
    (:else
      _))
  (Variables|Default|SetDialoguePlaying false)
  (bind _reponsewheelwidget (Variables|Default|GetReponseWheelWidget)
    (:then
      (Widget|RemovefromParent _reponsewheelwidget))
    (:else)))

(event Input|MouseEvents|RightMouseButton
  (params (Key :type Key%20Structure :default "None"))
  (:Pressed
    (if (Variables|Default|GetDialoguePlaying) :!label _label
      (bind _dialoguewheelwidget (Variables|Default|GetDialogueWheelWidget)
        (:then
          (Default|PlayerRightClick _dialoguewheelwidget))
        (:else))))
  (:Released
    (goto _label)))

(event Input|KeyboardEvents|L
  (params (Key :type Key%20Structure :default "None"))
  (:Pressed
    (Class|FarmerController|GameLost "Cow die")))

(event Input|MouseEvents|LeftMouseButton
  (params (Key :type Key%20Structure :default "None"))
  (:Pressed
    (if (Variables|Default|GetDialoguePlaying) :!label _label
      (bind _dialoguewheelwidget (Variables|Default|GetDialogueWheelWidget)
        (:then
          (Default|PlayerLeftClick _dialoguewheelwidget))
        (:else))))
  (:Released
    (goto _label)))

(fn ConstructionScript)

(fn ProcessMovetoFrontOfCow
  (bind _returnvalue (Game|GetPlayerCharacter 0))
  (bind _returnvalue_2 (Game|GetPlayerCharacter 0))
  (bind _closestcow (Variables|Default|GetClosestCow))
  (bind _returnvalue_3 (Transformation|GetActorLocation _closestcow))
  (bind _returnvalue_4 (Transformation|GetActorLocation _returnvalue))
  (bind _returnvalue_5 (Transformation|GetActorRotation _returnvalue_2))
  (bind _returnvalue_6 (Math|Rotator|FindLookatRotation _returnvalue_4 _returnvalue_3))
  (if (not (Variables|Default|GetHasReachedDestination))
    (if (Math|Vector|Equal(Vector) (Variables|Default|GetTargetDestination) (Transformation|GetActorLocation (Game|GetPlayerCharacter 0)) (Variables|Default|GetErrorToleranceInFrontOfCow))
      (if (Math|Rotator|Equal(Rotator) _returnvalue_5 _returnvalue_6 0.5)
        (Variables|Default|SetHasReachedDestination true)
        (else
          (Transformation|SetActorRotation _returnvalue (Math|Rotator|Lerp(Rotator) _returnvalue_5 _returnvalue_6 0.1)))))))