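; FarmerPlayerBP is the player farmer, handling cow interaction prompts and carrying hay.
; A looping timer tracks the closest cow and hides the previous cow's InteractLabel when the closest changes.
; Within range, the label's opacity fades in with proximity through a clamped distance remap.
; When the hay pickup event fires, CurrentHoldingHay attaches to the mesh's right-hand socket with a positional offset.
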(event Custom|EventDisplayCowInteractLabel
  (bind _returnvalue (Class|FarmerPlayer|GetClosestCow))
  (if (!= (Variables|Default|GetClosestCow) _returnvalue)
    (bind _ascow_bp (Utilities|Casting|CastToCowBP (Variables|Default|GetClosestCow))
      (:then
        (Widget|SetRenderOpacity (Variables|/Game/Gameplay/CowBP.CowBP_C|GetInteractLabel _ascow_bp) 0.0))
      (:CastFailed
        _)))
  (Variables|Default|SetClosestCow _returnvalue)
  (if (<= (Transformation|GetDistanceTo (Variables|Default|GetClosestCow)) 2.5e+02)
    (bind _ascow_bp_2 (Utilities|Casting|CastToCowBP (Variables|Default|GetClosestCow)))
    (Widget|SetRenderOpacity (Variables|/Game/Gameplay/CowBP.CowBP_C|GetInteractLabel _ascow_bp_2) (Math|Float|MapRangeClamped (Transformation|GetDistanceTo (Variables|Default|GetClosestCow)) 1e+02 2.5e+02 1.0 0.0))))

(event EventBeginPlay
  (Utilities|Time|SetTimerbyEvent (delegate Custom|EventDisplayCowInteractLabel) 0.05 true))

(event EventBIonPickedUpHay
  (bind _currentholdinghay (Variables|Default|GetCurrentHoldingHay))
  (Transformation|AttachComponentToComponent _currentholdinghay (Variables|Character|GetMesh) "hand_r" "KeepRelative" "KeepRelative" "KeepRelative" true)
  (Transformation|SetActorRelativeLocation _currentholdinghay "-15.000000,10.000000,0.000000"))

(fn ConstructionScript)