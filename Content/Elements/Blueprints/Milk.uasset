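; Milk is a short-lived actor that shrinks while drifting toward the player character, then destroys itself.
; On BeginPlay, the LifeSpan timeline plays in reverse from its end, driving uniform scale and a small location lerp toward player 0 on each update.
; The timeline's finish destroys the actor directly; a branch that toggles the particle effect and delays destruction to let it fade is disconnected.
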(event EventTick
  (params (DeltaSeconds :type Float%20%28single-precision%29)))

(event EventBeginPlay
  (bind _scale (Timeline|LifeSpan ReverseFromEnd) ; Timeline blends from 1 to 0.15
    (:Update
      (Transformation|SetActorRelativeScale3D (* (Math|Vector|MakeVector 1.0 1.0 1.0) _scale)) ; Gradually shrink the actor
      (Transformation|SetActorLocation (Math|Vector|Lerp(Vector) (Transformation|GetActorLocation) (Transformation|GetActorLocation (Game|GetPlayerCharacter 0)) 0.01) false false))
    (:Finished
      (Actor|DestroyActor))))

(fn ConstructionScript)